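; Actor component that syncs its BuildingData with a local MySQL buildings table, intended to trigger on cursor-over of its owner.
; Each hover toggles IsClicked; toggling on connects, runs a SELECT by building name, then inserts through string-formatted SQL.
; The insert depends on the InBldgTable field, as the SELECT result is unused.
; The cursor binding and StaticMeshRef setup are disconnected, so nothing here triggers the handler.
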(event Custom|OnCursorOver
  (params (TouchedActor :type Actor%20Object%20Reference))
  (bind _buildingdata (Variables|Default|GetBuildingData))
  (bind (_buildingname _departmentname _isdepartment _inbldgtable) (Utilities|Struct|BreakBS_BuildingInfo _buildingdata))
  ;[1 1 1] SELECT BUILDING DATA FROM DATABASE
  (bind _output_get (Variables|Default|SetIsClicked (not (Variables|Default|GetIsClicked))))
  (Utilities|IsValid (Variables|Default|GetStaticMeshRef)
    (:Is%20Valid
      (if _output_get
        (bind _connection (Utilities|MySQLConnect "localhost" "root" "" "capstonedb")
          (:Success
            (Utilities|MySQLExecuteQuery (Utilities|String|ToString(Text) (Utilities|Text|FormatText "SELECT * FROM buildingtbl where building_name='{BuildingName}';" (.BuildingName (Utilities|Struct|BreakBS_BuildingInfo (Variables|Default|GetBuildingData))))) _connection
              (:Success
                (for _array_element (Utilities|Array|MakeArray (Variables|Default|GetBuildingData))
                  (bind _output_get_2 (Variables|Default|SetArray%20Element _array_element))
                  (if (== 0 (.InBldgTable (Utilities|Struct|BreakBS_BuildingInfo _output_get_2)))
                    (Development|PrintString "Alraedy exiust")
                    (else
                      (Utilities|MySQLExecuteQuery (Utilities|String|ToString(Text) (Utilities|Text|FormatText "INSERT INTO buildingtbl (in_bldgtable, building_name, department_name, is_department) VALUES ( '{InBldgTable}', '{BuildingData}', '{DepartmentName}', '{IsDepartment}');" _inbldgtable _buildingname _departmentname _isdepartment)) _connection
                        (:Success
                          (Development|PrintString (Utilities|String|ToString(Integer) (.InBldgTable (Utilities|Struct|BreakBS_BuildingInfo (Variables|Default|GetBuildingData))))))))))))))))))

(event EventBeginPlay
  ;[1 1 1] SELECT BUILDING DATA FROM DATABASE
)

(event EventTick
  (params (DeltaSeconds :type Float%20%28single-precision%29))
  ;[1 1 1] SELECT BUILDING DATA FROM DATABASE
)