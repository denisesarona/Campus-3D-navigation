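; Blueprint functions that query a local MySQL capstone database for department records and create WB_BaseButton widgets from the results.
; RetrieveAllDatabaseData selects all departments and calls CreateBtns per row, which adds placeholder-text buttons to the viewport.
; SimpleQuery opens its own connection and creates a button per name field, but clears its text and never displays it.
; MySQLConnection only opens the connection, and the DeptArray assignment is unwired.
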(fn RetrieveAllDatabaseData
  ;[1 1 1] MySQL Function to retrieve All Data from Database
  (Utilities|MySQLExecuteQuerywithResult "SELECT * FROM departmenttb"
    (:Success
      (for _array_element 0
        (CallFunction|CreateBtns)))))

(fn CreateBtns
  ;[1 1 1] Function to Create Buttons
  (bind _returnvalue (UserInterface|CreateWidget "/Game/Widgets/WB_BaseButton.WB_BaseButton_C" 0 "Button Text"))
  (UserInterface|Viewport|AddtoViewport _returnvalue 0))

(fn SimpleQuery
  (bind _connection (Utilities|MySQLConnect "localhost" "root" "" "capstonedb")
    (:Success
      (bind _returnvalue (Class|MySQLDatabase|MySQLConnectorGetData "SELECT name FROM departmenttb" _connection))
      (for _array_element (.ResultRows (Utilities|Struct|BreakMySQLConnectoreQueryResult _returnvalue))
        (for _array_element_2 (Utilities|Struct|BreakMySQLConnectorQueryResultRow _array_element)
          (bind _returnvalue_2 (UserInterface|CreateWidget "/Game/Widgets/WB_BaseButton.WB_BaseButton_C" 0 (Utilities|Text|ToText(String) (.Value (Utilities|Struct|BreakMySQLConnectorKeyValuePair _array_element_2)))))
          (Variables|/Game/Widgets/WB_BaseButton.WB_BaseButton_C|SetButtonText _returnvalue_2 ""))))))

(fn MySQLConnection
  (Utilities|MySQLConnect "localhost" "root" "" "capstonedb"))